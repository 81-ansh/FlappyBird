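; BP_FBGameMode is the game mode for a bird game, handling the high score save and the game-over flow.
; On BeginPlay it loads or creates the BP_HighScore save in a single slot, then adds the HUD widget.
; When the bird dies, it saves any new high score, then after a short delay pauses the game and shows the game-over widget with UI-only input and a mouse cursor.
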(event `self.ReceiveBeginPlay`
  (bind _returnvalue (`GameplayStatics.GetPlayerController` 0))
  (bind _returnvalue_2 (`GameplayStatics.DoesSaveGameExist` "1"))
  (if _returnvalue_2
    (bind _returnvalue_3 (`GameplayStatics.LoadGameFromSlot` "1"))
    (bind _asbp_high_score (cast `/Game/Blueprints/Game/BP_HighScore` _returnvalue_3))
    (set `self.HighScoreRef` _asbp_high_score)
    (else
      (bind _returnvalue_4 (`GameplayStatics.CreateSaveGameObject` "/Game/Blueprints/Game/BP_HighScore.BP_HighScore_C"))
      (bind _output_get (set `self.HighScoreRef` _returnvalue_4))
      (`GameplayStatics.SaveGameToSlot` _output_get "1")))
  (set `self.PlayerController` _returnvalue)
  (bind _returnvalue_5 (`|CreateWidget` "/Game/Blueprints/UI/WBP_HUD.WBP_HUD_C" _returnvalue))
  (`UserWidget.AddToViewport` _returnvalue_5 0))

(event `self.OnBirdDied`
  (bind _returnvalue (`GameplayStatics.GetPlayerController` 0))
  (bind _highscoreref (`self.HighScoreRef`))
  (if (> (`self.Score`) (`/Game/Blueprints/Game/BP_HighScore.HighScore` (`self.HighScoreRef`)))
    (set `/Game/Blueprints/Game/BP_HighScore.HighScore` (`self.Score`) _highscoreref)
    (`GameplayStatics.SaveGameToSlot` _highscoreref "1"))
  (`KismetSystemLibrary.Delay` 0.5)
  (`GameplayStatics.SetGamePaused` true)
  (bind _returnvalue_2 (`|CreateWidget` "/Game/Blueprints/UI/WBP_GameOver.WBP_GameOver_C" _returnvalue))
  (`UserWidget.AddToViewport` _returnvalue_2 0)
  (`WidgetBlueprintLibrary.SetInputMode_UIOnlyEx` _returnvalue _returnvalue_2)
  (set `PlayerController.bShowMouseCursor` true _returnvalue))

(fn `UserConstructionScript`)